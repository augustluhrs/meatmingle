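; Test OSC manager actor that opens a listening OSC server named "TouchDesigner" on a configurable IP and port at BeginPlay.
; It binds a handler for any received message, which currently only prints "Hello" alongside a lookup on a newly made empty bundle.
; Address and value parsing with a 1/0 debug branch is left disconnected, and the bundle-received event is empty.
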(event Custom|OnMsgReceived
  (params (Message :type OSC%20Message%20Structure%20%28by%20ref%29) (IPAddress :type String) (Port :type Integer))
  ;[1 1 1] Binding to Any Message
  (Class|OSCManager|GetMessagefromBundle (Utilities|Struct|MakeOSCBundle))
  (Development|PrintString "Hello"))

(event Custom|OnBundleReceived
  ;[1 1 1] Binding to Any Message
)

(event EventBeginPlay
  ;[1 1 1] Binding to Any Message
  (bind _returnvalue (Class|OSCManager|CreateOSCServer (Variables|Default|GetReceive%20IPAddress) (Variables|Default|GetPort) false true "TouchDesigner" 0))
  (bind _output_get (Variables|Default|SetOSCServer _returnvalue))
  (EventDispatchers|AssignOnOscMessageReceived _output_get (delegate Custom|OnMsgReceived)))

(event Collision|EventActorBeginOverlap
  (params (OtherActor :type Actor%20Object%20Reference)))

(event EventTick
  (params (DeltaSeconds :type Float%20%28single-precision%29)))

(fn ConstructionScript)